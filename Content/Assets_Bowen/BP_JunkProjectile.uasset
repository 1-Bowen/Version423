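; Junk projectile actor that explodes two seconds after spawning, or sooner if its Sphere1 component hits an actor tagged "Junk".
; Both triggers call a shared Explode function, which spawns an emitter at the projectile's location, plays a quieter 2D sound and destroys the actor.
; The Blueprint applies no damage and leaves the hit actor untouched.
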(event OnComponentHit(Sphere1)
  (params (HitComponent :type Primitive%20Component%20Object%20Reference) (OtherActor :type Actor%20Object%20Reference) (OtherComp :type Primitive%20Component%20Object%20Reference) (NormalImpulse :type Vector :default "0, 0, 0") (Hit :type Hit%20Result%20Structure%20%28by%20ref%29))
  (if (Actor|ActorHasTag OtherActor "Junk")
    (CallFunction|Explode)))

(event EventBeginPlay
  (Utilities|FlowControl|Delay 2.0)
  (CallFunction|Explode))

(event Collision|EventActorBeginOverlap
  (params (OtherActor :type Actor%20Object%20Reference)))

(event EventTick
  (params (DeltaSeconds :type Float%20%28single-precision%29)))

(fn ConstructionScript)

(fn Explode
  (Effects|SpawnEmitteratLocation 0 (Transformation|GetActorLocation))
  (Audio|PlaySound2D 0 0.4 1.0 0.0 0 0)
  (Actor|DestroyActor))